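; Player controller for a party of pawns tagged "Playable", switching possession by cycling or number keys and toggling first-person camera mode.
; On start it gathers the pawns, creates a selection widget and builds a dynamic post-process noise material.
; Non-instant switches play a timer-driven, curve-shaped static effect, delaying possession until halfway through.
; Possession retargets FollowingCharacterAI controllers to the new leader and reapplies the shared camera mode.
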(event EventBeginPlay
  (CallFunction|FillListwithCharacters)
  (CallFunction|AddWidget)
  (CallFunction|SetupPostProcessComponent)
  (CallFunction|PossessCharacter 0 true))

(event Input|ActionEvents|InputActionSwitchCharacter
  (params (Key :type Key%20Structure :default "None"))
  (:Pressed
    (CallFunction|PossessNextCharacter)))

(event Input|ActionEvents|InputActionSwitchCamera
  (params (Key :type Key%20Structure :default "None"))
  (:Pressed
    (CallFunction|ChangeCameraMode)))

(event Input|KeyboardEvents|1
  (params (Key :type Key%20Structure :default "None"))
  (:Pressed
    (CallFunction|PossessCharacter 0 false)))

(event Input|KeyboardEvents|2
  (params (Key :type Key%20Structure :default "None"))
  (:Pressed
    (CallFunction|PossessCharacter 1 false)))

(event Input|KeyboardEvents|3
  (params (Key :type Key%20Structure :default "None"))
  (:Pressed
    (CallFunction|PossessCharacter 2 false)))

(event Input|KeyboardEvents|4
  (params (Key :type Key%20Structure :default "None"))
  (:Pressed
    (CallFunction|PossessCharacter 3 false)))

(event Input|KeyboardEvents|5
  (params (Key :type Key%20Structure :default "None"))
  (:Pressed
    (CallFunction|PossessCharacter 4 false)))

(fn ConstructionScript)

(fn SetupPostProcessComponent
  (bind _noisepostprocess (Variables|Default|GetNoisePostprocess))
  (bind _returnvalue (Rendering|Material|CreateDynamicMaterialInstance "/Game/Materials/StaticPostProcesMat.StaticPostProcesMat" "None" :!class /Script/Engine.KismetMaterialLibrary))
  (bind _output_get (Variables|StaticEffect|SetNoiseMaterial _returnvalue))
  (Rendering|Material|SetScalarParameterValue _output_get "postprocessLevel" 0.0 :!class /Script/Engine.MaterialInstanceDynamic)
  (bind _structout (Utilities|Struct|SetmembersinPostProcessSettings (Variables|/Script/Engine.PostProcessComponent|GetSettings _noisepostprocess) (Utilities|Struct|MakeWeightedBlendables (Utilities|Array|MakeArray (Utilities|Struct|MakeWeightedBlendable 1.0 (Variables|StaticEffect|GetNoiseMaterial))))))
  (Variables|/Script/Engine.PostProcessComponent|SetSettings _noisepostprocess _structout))

(fn StartStaticNoise
  (bind _returnvalue (Utilities|Time|SetTimerbyEvent (EventDispatchers|CreateEvent :!event UpdateStaticNoise) (Variables|StaticEffect|GetNoiseEffectStepSize) true))
  (Variables|StaticEffect|SetNoiseTimerHandle _returnvalue)
  (Rendering|SetVisibility (Variables|Default|GetNoisePostprocess) true false))

(fn UpdateStaticNoise
  (if (>= (Variables|StaticEffect|GetNoiseElapsedTime) (Variables|StaticEffect|GetNoiseDuration))
    (Utilities|Time|ClearandInvalidateTimerbyHandle (Variables|StaticEffect|GetNoiseTimerHandle))
    (bind _output_get (Variables|StaticEffect|SetNoiseElapsedTime 0.0))
    (Rendering|Material|SetScalarParameterValue (Variables|StaticEffect|GetNoiseMaterial) "postprocessLevel" _output_get :!class /Script/Engine.MaterialInstanceDynamic)
    (Rendering|SetVisibility (Variables|Default|GetNoisePostprocess) false false)
    (else
      (Rendering|Material|SetScalarParameterValue (Variables|StaticEffect|GetNoiseMaterial) "postprocessLevel" (Math|Curves|GetFloatValue (Variables|StaticEffect|GetNoiseEffectCurve) (/ (Variables|StaticEffect|GetNoiseElapsedTime) (Variables|StaticEffect|GetNoiseDuration))) :!class /Script/Engine.MaterialInstanceDynamic)
      (Variables|StaticEffect|SetNoiseElapsedTime (+ (Variables|StaticEffect|GetNoiseElapsedTime) (Variables|StaticEffect|GetNoiseEffectStepSize))))))

(fn AddWidget
  (bind _returnvalue (UserInterface|CreateWidget "/Game/Blueprints/CharacterSelcetionUI.CharacterSelcetionUI_C"))
  (bind _output_get (Variables|Default|SetCharacterSelectionWidget _returnvalue))
  (UserInterface|Viewport|AddtoViewport _returnvalue 0)
  (Default|FillNames _output_get (Variables|Default|GetCharacters)))

(fn FillListwithCharacters
  (bind _outactors (Actor|GetAllActorsOfClasswithTag "/Script/Engine.Pawn" "Playable"))
  (Variables|Default|SetCharacters _outactors))

(fn UpdateWidget
  (Default|SetActiveCharacter (Variables|Default|GetCharacterSelectionWidget) (Variables|Default|GetCharacterIndex)))

(fn PossessNextCharacter
  (CallFunction|PossessCharacter (Math|Integer|%(Integer) (+ (Variables|Default|GetCharacterIndex) 1) (Utilities|Array|Length (Variables|Default|GetCharacters))) false))

(fn PossessCharacter
  (params (NewCharacterIndex :type Integer) (isInstant :type Boolean))
  (if (!= NewCharacterIndex (Variables|Default|GetCharacterIndex))
    (Variables|Default|SetCharacterIndex (Math|Integer|%(Integer) NewCharacterIndex (Utilities|Array|Length (Variables|Default|GetCharacters))))
    (if (or isInstant (Utilities|Time|IsValidTimerHandle (Variables|StaticEffect|GetNoiseTimerHandle)))
      (CallFunction|FinishPossessCharacter)
      (else
        (Utilities|Time|SetTimerbyEvent (EventDispatchers|CreateEvent :!event FinishPossessCharacter) (/ (Variables|StaticEffect|GetNoiseDuration) 2.0))
        (CallFunction|StartStaticNoise)))
    (CallFunction|UpdateWidget)))

(fn FinishPossessCharacter
  (bind _characterindex (Variables|Default|GetCharacterIndex))
  (bind _characters (Variables|Default|GetCharacters))
  (bind _output (Utilities|Array|Get(acopy) _characters _characterindex))
  (Pawn|Possess _output)
  (for _array_element (Variables|Default|GetCharacters)
    (bind _asfollowing_character_ai (Utilities|Casting|CastToFollowingCharacterAI (Pawn|GetController _array_element)))
    (Default|SetNewLeader _asfollowing_character_ai _output))
  (CallFunction|SetCameraMode))

(fn ChangeCameraMode
  (Variables|Default|SetisFPP (not (Variables|Default|GetisFPP)))
  (CallFunction|SetCameraMode))

(fn SetCameraMode
  (bind _asthird_person_character (Utilities|Casting|CastToThirdPersonCharacter (Utilities|Array|Get(acopy) (Variables|Default|GetCharacters) (Variables|Default|GetCharacterIndex))))
  (Default|SetCameraMode _asthird_person_character (Variables|Default|GetisFPP)))